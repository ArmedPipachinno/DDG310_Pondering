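; Goldfish AI character that loops a swim animation and serves as a shootable target in the FishWithGun game mode.
; Point damage feeds AiHP; a true result destroys the fish, adds FastFish to the game mode's Coin and calls CheckWinLose.
; Projectile overlaps on the capsule randomly trigger a jump and MoveComponentTo, with debug prints.
; Movement and spawner experiments remain in the graph but are never run.
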(event `self.ReceiveBeginPlay`
  (`SkeletalMeshComponent.PlayAnimation` (`self.Mesh`) "/Game/Assets/Fish_Schools/Fish_School_Goldfish/Models/Goldfish__Swim.Goldfish__Swim" true))

(event `self.ReceiveTick`
  (params (DeltaSeconds :type "Float (single-precision)")))

(event `self.ReceivePointDamage`
  (params (Damage :type "Float (single-precision)") (DamageType :type "DamageType Object Reference") (HitLocation :type "Vector Structure") (HitNormal :type "Vector Structure") (HitComponent :type "PrimitiveComponent Object Reference") (BoneName :type Name) (ShotFromDirection :type "Vector Structure") (InstigatedBy :type "Controller Object Reference") (DamageCauser :type "Actor Object Reference") (HitInfo :type "HitResult Structure (by ref)"))
  (bind _capsulecomponent (`self.CapsuleComponent`))
  (`KismetSystemLibrary.PrintString` (`KismetStringLibrary.Conv_DoubleToString` Damage))
  (bind _isdead (`/Game/Blueprint/AI_BP/Ai_HP.TakeDamage` (`self.Ai_HP`) Damage))
  (if _isdead
    (`MovementComponent.StopMovementImmediately` (`self.CharacterMovement`))
    (`self.SetLifeSpan` (`self.In Lifespan`))
    (`PrimitiveComponent.SetCollisionResponseToChannel` _capsulecomponent "ECC_WorldStatic" "ECR_Ignore")
    (`PrimitiveComponent.SetCollisionResponseToChannel` _capsulecomponent "ECC_Pawn" "ECR_Ignore")
    (`self.DetachFromControllerPendingDestroy`)
    (`self.K2_DestroyActor`)
    (bind _asfish_with_gun (cast `/Game/Blueprint/FishWithGun` (`GameplayStatics.GetGameMode`)))
    (set `/Game/Blueprint/FishWithGun.Coin` (+ (`/Game/Blueprint/FishWithGun.Coin` _asfish_with_gun) (`self.Fast Fish`)) _asfish_with_gun)
    (bind _asfish_with_gun_2 (cast `/Game/Blueprint/FishWithGun` (`GameplayStatics.GetGameMode`)))
    (`/Game/Blueprint/FishWithGun.Check Win lose` _asfish_with_gun_2)))

(event `self.CapsuleComponent.OnComponentBeginOverlap`
  (params (OverlappedComponent :type "PrimitiveComponent Object Reference") (OtherActor :type "Actor Object Reference") (OtherComp :type "PrimitiveComponent Object Reference") (OtherBodyIndex :type Integer) (bFromSweep :type Boolean) (SweepResult :type "HitResult Structure (by ref)"))
  (bind _returnvalue (`KismetMathLibrary.RandomInteger` 11))
  (cast `/Game/Blueprint/Weapons_BP/Projectile` OtherActor)
  (`KismetSystemLibrary.PrintString` (`KismetStringLibrary.Conv_IntToString` _returnvalue))
  (if (== _returnvalue 0)
    (`KismetSystemLibrary.PrintString` "Jump")
    (`self.Jump`)
    (`KismetSystemLibrary.MoveComponentTo` null)
    (else
      (`KismetSystemLibrary.PrintString` "FAil"))))

(event `self.CapsuleComponent.OnComponentHit`
  (params (HitComponent :type "PrimitiveComponent Object Reference") (OtherActor :type "Actor Object Reference") (OtherComp :type "PrimitiveComponent Object Reference") (NormalImpulse :type "Vector Structure") (Hit :type "HitResult Structure (by ref)")))

(fn `UserConstructionScript`)