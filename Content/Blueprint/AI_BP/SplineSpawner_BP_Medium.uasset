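; Spline spawner actor that keeps spawning AI goldfish and moves them along a looping spline path.
; On BeginPlay, a self-repeating delayed event spawns fish at the Billboard's location and adds them to an array, with no cap.
; A replaying timeline, rate-scaled by its length setting, sets each fish's location and rotation along the spline, staggered by array index and wrapped past the end.
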(event `self.ReceiveBeginPlay`
  (`TimelineComponent.SetPlayRate` (`self.SplineMoverTimeLine`) (/ (`self.PlayRate`) (`self.TimeLineLenght`)))
  (`self.SpawnFishInArray`)
  (`self.PlayTimeline`))

(event `SpawnFishInArray`
  (bind _fish_spawn_duration (`self.Fish spawn duration`))
  (for _ (range 2)
    (`KismetSystemLibrary.Delay` _fish_spawn_duration)
    (bind _returnvalue (`AIBlueprintHelperLibrary.SpawnAIFromClass` "/Game/Blueprint/AI_BP/Simple_AI_Goldfish_2.Simple_AI_Goldfish_2_C" null (`SceneComponent.K2_GetComponentLocation` (`self.Billboard`)) (struct) false null))
    (`KismetArrayLibrary.Array_Add` (`self.Actor`) _returnvalue))
  (`KismetSystemLibrary.Delay` _fish_spawn_duration)
  (`self.SpawnFishInArray`))

(event `PlayTimeline`
  (bind _spline (`self.Spline`))
  (bind _distancealongspline (`self.DistanceAlongSpline`))
  (bind _returnvalue (`SplineComponent.GetSplineLength` (`self.Spline`)))
  ;[1 1 1] Spline movement
  (bind (_direction _spm_alpha) (`Timeline|SplineMoverTimeLine` :`NewTime` 100.0 :!via `PlayFromStart`)
    (:`Update`
      (for (_array_element _array_index) (`self.Actor`)
        (bind _output_get (set `self.DistanceAlongSpline` (+ (`KismetMathLibrary.Lerp` 0.0 (`SplineComponent.GetSplineLength` (`self.Spline`)) _spm_alpha) (* _array_index (`self.ActorOffset`)))))
        (if (> _output_get _returnvalue)
          (set `self.DistanceAlongSpline` (- (`self.DistanceAlongSpline`) _returnvalue)))
        (`self.K2_SetActorLocationAndRotation` _array_element (`SplineComponent.GetLocationAtDistanceAlongSpline` _spline _distancealongspline "World") (`SplineComponent.GetRotationAtDistanceAlongSpline` _spline _distancealongspline "World") false false)))
    (:`Finished`
      (`self.PlayTimeline`))))

(fn `UserConstructionScript`
  (bind _spline (`self.Spline`))
  (for (_ _array_index) (`self.Actor`)
    (bind _returnvalue (* _array_index (`self.ActorOffset`)))
    (`self.K2_SetActorLocationAndRotation` (`SplineComponent.GetLocationAtDistanceAlongSpline` _spline _returnvalue "World") (`SplineComponent.GetRotationAtDistanceAlongSpline` _spline _returnvalue "World"))))