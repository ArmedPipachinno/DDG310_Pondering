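; Spline mover Blueprint that loops an array of actors continuously along its spline, matching their position and rotation to the path.
; A self-restarting timeline, with its rate set from PlayRate and length, maps alpha to spline distance.
; Each actor adds an index-based offset, wrapping once past the spline's end.
; The construction script computes the same spaced transforms but applies them to the Blueprint itself, not the array's actors.
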(event `self.ReceiveBeginPlay`
  (`TimelineComponent.SetPlayRate` (`self.SplineMoverTimeLine`) (/ (`self.PlayRate`) (`self.TimeLineLenght`)))
  (`self.PlayTimeline`))

(event `PlayTimeline`
  (bind _spline (`self.Spline`))
  (bind _distancealongspline (`self.DistanceAlongSpline`))
  (bind _returnvalue (`SplineComponent.GetSplineLength` (`self.Spline`)))
  (bind (_direction _spm_alpha) (`Timeline|SplineMoverTimeLine` :`NewTime` 100.0 :!via `PlayFromStart`)
    (:`Update`
      (for (_array_element _array_index) (`self.Actor`)
        (bind _output_get (set `self.DistanceAlongSpline` (+ (`KismetMathLibrary.Lerp` 0.0 (`SplineComponent.GetSplineLength` (`self.Spline`)) _spm_alpha) (* _array_index (`self.ActorOffset`)))))
        (if (> _output_get _returnvalue)
          (set `self.DistanceAlongSpline` (- (`self.DistanceAlongSpline`) _returnvalue)))
        (`self.K2_SetActorLocationAndRotation` _array_element (`SplineComponent.GetLocationAtDistanceAlongSpline` _spline _distancealongspline "World") (`SplineComponent.GetRotationAtDistanceAlongSpline` _spline _distancealongspline "World") false false)))
    (:`Finished`
      (`self.PlayTimeline`))))

(fn `UserConstructionScript`
  (bind _spline (`self.Spline`))
  (for (_ _array_index) (`self.Actor`)
    (bind _returnvalue (* _array_index (`self.ActorOffset`)))
    (`self.K2_SetActorLocationAndRotation` (`SplineComponent.GetLocationAtDistanceAlongSpline` _spline _returnvalue "World") (`SplineComponent.GetRotationAtDistanceAlongSpline` _spline _returnvalue "World"))))