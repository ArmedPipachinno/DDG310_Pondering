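; Field_Agent is a player-controlled pawn with a fish mesh that turns, walks and attacks at short range.
; Axis inputs drive controller yaw and move the pawn along that yaw.
; Shoot runs a debug-drawn multi sphere trace forward from FishMesh, printing and applying point damage to each hit, credited to player 0.
; An older capsule-trace damage path remains disconnected and never runs.
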(event `InputAxis|X-axis`
  (params (AxisValue :type "Float (single-precision)"))
  (`self.AddControllerYawInput` AxisValue))

(event `InputAxis|walk`
  (params (AxisValue :type "Float (single-precision)"))
  (`self.AddMovementInput` (`KismetMathLibrary.GetForwardVector` (`KismetMathLibrary.MakeRotator` 0.0 0.0 (.yaw (`self.GetControlRotation`)))) AxisValue))

(event `InputAction|Shoot`
  (params (Key :type "Key Structure"))
  (bind _fishmesh (`self.FishMesh`))
  (bind _returnvalue (`SceneComponent.K2_GetComponentLocation` _fishmesh))
  (:`Pressed`
    (bind _outhits (`KismetSystemLibrary.SphereTraceMulti` :`Start` _returnvalue :`End` (+ _returnvalue (* (`SceneComponent.GetForwardVector` _fishmesh) 200.0)) :`Radius` 75.0 :`TraceChannel` "TraceTypeQuery2" :`DrawDebugType` "ForDuration"))
    (for _array_element _outhits
      (if true
        (bind (_bblockinghit _binitialoverlap _time _distance _location _impactpoint _normal _impactnormal _physmat _hitactor _hitcomponent _hitbonename _hititem _elementindex _faceindex _tracestart) (`GameplayStatics.BreakHitResult` _array_element))
        (`KismetSystemLibrary.PrintString` (`KismetSystemLibrary.GetDisplayName` _hitactor))
        (`GameplayStatics.ApplyPointDamage` _hitactor 50.0 _tracestart _array_element (`GameplayStatics.GetPlayerController` 0))))))

(fn `UserConstructionScript`)