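; FishWithGun Blueprint that holds the win and lose check for the game, based on a Coin count.
; Its CheckWinlose event opens the WinMenu level once, through a DoOnce, when Coin reaches WinGoal, and reloads the current level when Coin drops to zero or below.
; Tick, BeginPlay and the construction script are empty, and nothing in this file calls the check or changes Coin.
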(event `self.ReceiveTick`
  (params (DeltaSeconds :type "Float (single-precision)")))

(event `Check Win lose`
  (if (>= (`self.Coin`) (`self.Win goal`))
    (`/Engine/EditorBlueprintResources/StandardMacros.DoOnce` false
      (:`Completed`
        (`KismetSystemLibrary.PrintString` "Winning Son")
        (`GameplayStatics.OpenLevel` "WinMenu")))
    (elif (<= (`self.Coin`) 0)
      (bind _returnvalue (`GameplayStatics.GetCurrentLevelName` true))
      (`GameplayStatics.OpenLevel` (`KismetStringLibrary.Conv_StringToName` _returnvalue)))))

(fn `UserConstructionScript`)